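; BP_ClearItem is a level-clear pickup that sends the player to the next numbered room.
; It spins slightly every Tick, at a frame-rate-dependent speed.
; When BP_ThirdPersonCharacter overlaps its StaticMesh, it parses the last two characters of the current level name, adds one, opens the zero-padded "Room_NN" level, then destroys itself.
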(event OnComponentBeginOverlap(StaticMesh)
  (params (OverlappedComponent :type Primitive%20Component%20Object%20Reference) (OtherActor :type Actor%20Object%20Reference) (OtherComp :type Primitive%20Component%20Object%20Reference) (OtherBodyIndex :type Integer) (bFromSweep :type Boolean) (SweepResult :type Hit%20Result%20Structure%20%28by%20ref%29))
  (Utilities|Casting|CastToBP_ThirdPersonCharacter OtherActor)
  (bind _returnvalue (Game|GetCurrentLevelName true))
  (Game|OpenLevel(byName) (Utilities|String|StringToName (Utilities|String|Append "Room_" (Utilities|String|ToString(Text) (Utilities|Text|ToText(Integer) (+ (Math|Conversions|ToInteger(Byte) (Utilities|String|Right _returnvalue 2)) 1) false false 2)))))
  (Actor|DestroyActor))

(event EventBeginPlay)

(event Collision|EventActorBeginOverlap
  (params (OtherActor :type Actor%20Object%20Reference)))

(event EventTick
  (params (DeltaSeconds :type Float%20%28single-precision%29))
  (Transformation|AddActorLocalRotation "0.000000,0.500000,0.000000" false false))

(fn ConstructionScript)